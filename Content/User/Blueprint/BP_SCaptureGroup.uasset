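; BP_SCaptureGroup is an actor that slowly sweeps its CaptureComp back and forth along its local Y axis.
; On BeginPlay a slowed Timeline drives a Lerp that sets the component's relative location between two fixed offsets.
; When the Timeline finishes, a playback-position check either plays or reverses it, producing an endless ping-pong motion.
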(event `self.ReceiveBeginPlay`
  (bind _timeline (`self.Timeline`))
  (`TimelineComponent.SetPlayRate` (`self.Timeline`) 0.1)
  (bind (_direction _alpha) (`Timeline|Timeline`)
    (:`Update`
      (`SceneComponent.K2_SetRelativeLocation` (`self.CaptureComp`) (`KismetMathLibrary.MakeVector` 0.0 (`KismetMathLibrary.Lerp` -1000.0 1000.0 _alpha)) false false))
    (:`Finished`
      (if (== (`TimelineComponent.GetPlaybackPosition` _timeline) 0.0)
        (`TimelineComponent.Play` _timeline)
        (else
          (`TimelineComponent.Reverse` _timeline))))))

(fn `UserConstructionScript`)